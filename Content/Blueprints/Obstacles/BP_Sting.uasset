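; BP_Sting is an obstacle that pops and destroys the player's balloon pawn on contact.
; A Box overlap with player pawn 0 calls Destroy, which casts to BalloonPawn_BP, plays the Bang sound and puts a dynamic M_Flash material on the balloon mesh.
; A timeline animates that material's dissolve parameter, then removes the sound component and destroys the pawn when finished.
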(event OnComponentBeginOverlap(Box)
  (params (OverlappedComponent :type Primitive%20Component%20Object%20Reference) (OtherActor :type Actor%20Object%20Reference) (OtherComp :type Primitive%20Component%20Object%20Reference) (OtherBodyIndex :type Integer) (bFromSweep :type Boolean) (SweepResult :type Hit%20Result%20Structure%20%28by%20ref%29))
  (bind _returnvalue (Game|Player|GetPlayerPawn 0))
  (if (== OtherActor _returnvalue)
    ;[1 1 1] @To do:Destroy Effect
    (CallFunction|Destroy _returnvalue)))

(event Custom|Destroy
  (params (PlayerPawn :type Pawn%20Object%20Reference))
  ;[1 1 1] cast to player reference
  (bind _asballoon_pawn_bp (Utilities|Casting|CastToBalloonPawn_BP PlayerPawn))
  (bind _returnvalue (Audio|SpawnSound2D "/Game/Arts/Sounds/bang.bang" 1.0 1.0 0.0 0))
  (bind _returnvalue_2 (Rendering|Material|CreateDynamicMaterialInstance (Variables|/Script/Balloon.BalloonPawn|GetBalloonMesh _asballoon_pawn_bp) 0 "/Game/Arts/Materials/M_Flash.M_Flash" "None" :!class /Script/Engine.PrimitiveComponent))
  (bind _newtrack_0 (Timeline|Destory PlayFromStart)
    (:Update
      (Rendering|Material|SetScalarParameterValue _returnvalue_2 "消散" (Math|Float|Lerp 0.5 0.0 _newtrack_0) :!class /Script/Engine.MaterialInstanceDynamic))
    (:Finished
      (Components|DestroyComponent _returnvalue)
      (Actor|DestroyActor PlayerPawn))))

(event EventBeginPlay)

(event Collision|EventActorBeginOverlap
  (params (OtherActor :type Actor%20Object%20Reference)))

(event EventTick
  (params (DeltaSeconds :type Float%20%28single-precision%29)))

(fn ConstructionScript)