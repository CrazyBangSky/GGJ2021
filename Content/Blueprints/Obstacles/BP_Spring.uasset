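; BP_Spring is an obstacle that launches the player's balloon when it touches the spring.
; A Box overlap by the player's BalloonPawn_BP applies an impulse to its BalloonMesh along the Arrow's forward vector, scaled by ForceStrength.
; The impulse is a velocity change, so mass is ignored, and a 2D spring sound plays.
; Spring deformation is still a to-do.
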(event OnComponentBeginOverlap(Box)
  (params (OverlappedComponent :type Primitive%20Component%20Object%20Reference) (OtherActor :type Actor%20Object%20Reference) (OtherComp :type Primitive%20Component%20Object%20Reference) (OtherBodyIndex :type Integer) (bFromSweep :type Boolean) (SweepResult :type Hit%20Result%20Structure%20%28by%20ref%29))
  (bind _returnvalue (Game|Player|GetPlayerPawn 0))
  (if (== OtherActor _returnvalue)
    (bind _asballoon_pawn_bp (Utilities|Casting|CastToBalloonPawn_BP _returnvalue))
    (Physics|AddImpulse (Variables|/Script/Balloon.BalloonPawn|GetBalloonMesh _asballoon_pawn_bp) (* (Math|Vector|GetForwardVector (Variables|Default|GetArrow)) (Variables|GamePlayCustom|GetForceStrength)) "None" true)
    ;[1 1 1] @To Do:Spring deformation
    (Audio|PlaySound2D "/Game/Arts/Sounds/Spring.Spring" 1.0 1.0 0.0 0 0)))

(event EventBeginPlay)

(event Collision|EventActorBeginOverlap
  (params (OtherActor :type Actor%20Object%20Reference)))

(event EventTick
  (params (DeltaSeconds :type Float%20%28single-precision%29)))

(fn ConstructionScript)