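; BP_Wind is a wind zone obstacle that pushes the player's balloon and changes its heat.
; Each tick, while the player overlaps the box, it applies force along the arrow, scaled by strength and inverse distance, and calls ApplyHeat.
; The construction script selects cold or warm material and forward or back particles from flags.
; A wind sound spawned on BeginPlay fades linearly with player distance, updated every tick.
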(event Collision|EventActorBeginOverlap
  (params (OtherActor :type Actor%20Object%20Reference)))

(event EventTick
  (params (DeltaSeconds :type Float%20%28single-precision%29))
  (bind _returnvalue (Game|Player|GetPlayerPawn 0))
  (Utilities|FlowControl|Sequence
    (:then_0
      (for _array_element (Collision|GetOverlappingActors (Variables|Default|GetBox) "/Script/Engine.Pawn" :!class /Script/Engine.PrimitiveComponent)
        (if (== _array_element _returnvalue)
          ;[1 1 1] @To do:Add Force and Modify gas value
          (bind _asballoon_pawn_bp (Utilities|Casting|CastToBalloonPawn_BP _returnvalue))
          (Physics|AddForce (Variables|/Script/Balloon.BalloonPawn|GetBalloonMesh _asballoon_pawn_bp) (* (* (Math|Vector|GetForwardVector (Variables|Default|GetWindArrow)) (/ 1.0 (Math|Vector|Distance(Vector) (Transformation|GetWorldLocation (Variables|Default|GetBox)) (Transformation|GetWorldLocation (Variables|/Script/Balloon.BalloonPawn|GetBalloonMesh _asballoon_pawn_bp))))) (Variables|GamePlayCustom|GetStrength)) "None" false)
          (Class|BalloonPawn|ApplyHeat _asballoon_pawn_bp (* DeltaSeconds (Variables|GamePlayCustom|GetHeatValue))))))
    (:then_1
      (|PlayWindSound))))

(event EventBeginPlay
  (bind _returnvalue (Audio|SpawnSoundatLocation "/Game/Arts/Sounds/wind.wind" (Transformation|GetActorLocation) "0, 0, 0" 1.0 1.0 0.0 0 0))
  (Variables|Default|SetWIndSound _returnvalue))

(fn ConstructionScript
  (bind _particlesystem (Variables|Default|GetParticleSystem))
  (bind _particlesystem_2 (Variables|Default|GetParticleSystem))
  (Utilities|FlowControl|Sequence
    (:then_0
      (if (Variables|GamePlayCustom|GetIsClodWind)
        (Rendering|Material|SetMaterial _particlesystem 1 "/Game/Arts/Particles/Materials/M_ClodWind.M_ClodWind")
        (else
          (Rendering|Material|SetMaterial _particlesystem 1 "/Game/Arts/Particles/Materials/M_WarmWind.M_WarmWind"))))
    (:then_1
      (if (Variables|GamePlayCustom|GetIsForward)
        (Effects|Components|ParticleSystem|SetTemplate _particlesystem_2 "/Game/Arts/Particles/FX_ForwardWind.FX_ForwardWind")
        (else
          (Effects|Components|ParticleSystem|SetTemplate _particlesystem_2 "/Game/Arts/Particles/FX_Back_Wind.FX_Back_Wind"))))))