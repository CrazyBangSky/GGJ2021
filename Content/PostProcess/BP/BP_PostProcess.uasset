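; BP_PostProcess toggles cold and warm white balance shifts on the PPVDarktime post process volume.
; Each custom event uses a FlipFlop to alternately play its timeline and reverse it from the end.
; Timeline updates offset Temp down for cold or up for warm from a shared neutral base, printing the value for debugging.
; Both effects write the same setting independently, so they overwrite rather than blend.
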(event EventTemperatureCold
  (Utilities|FlowControl|FlipFlop
    (:A
      (bind _newtrack_0 (Timeline|Timeline_0 Play)
        (:Update
          (Utilities|Struct|SetmembersinPostProcessSettings (Variables|/Script/Engine.PostProcessComponent|GetSettings (Variables|Default|GetPPV_Darktime)) (+ (* _newtrack_0 -1e+03) 5.5e+03))
          (Development|PrintString (Utilities|String|ToString(Float) (+ (* _newtrack_0 -1e+03) 5.5e+03))))))
    (:B
      (Timeline|Timeline_0 ReverseFromEnd))))

(event EventTemperatureWarm
  (Utilities|FlowControl|FlipFlop
    (:A
      (bind _newtrack_0 (Timeline|Timeline_1 Play)
        (:Update
          (Utilities|Struct|SetmembersinPostProcessSettings (Variables|/Script/Engine.PostProcessComponent|GetSettings (Variables|Default|GetPPV_Darktime)) (+ (* _newtrack_0 2e+03) 5.5e+03))
          (Development|PrintString (Utilities|String|ToString(Float) (+ (* _newtrack_0 2e+03) 5.5e+03)) true true "(R=1.000000,G=0.026767,B=0.000000,A=1.000000)"))))
    (:B
      (Timeline|Timeline_1 ReverseFromEnd))))

(fn ConstructionScript)